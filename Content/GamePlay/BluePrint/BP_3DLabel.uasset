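; BP_3DLabel is a world-placed label actor that shows a named icon and serves as a camera focus point with optional surveillance video.
; Its construction script applies CameraData to a SpringArm and records the actor's location back into that struct.
; BeginPlay caches the player BP_Pawn and fills the WBP_3DIcon widget.
; ClickIcon plays any MediaSource through WBP_3DDetails, hiding the icon, then passes the camera data to the pawn to focus.
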(event EventBeginPlay
  (bind _cameradata (Variables|Default|GetCameraData))
  (Utilities|FlowControl|Sequence
    (:then_0
      (bind _asbp_pawn (Utilities|Casting|CastToBP_Pawn (Game|Player|GetPlayerPawn 0)))
      (Variables|Default|SetAs%20BP%20Pawn _asbp_pawn))
    (:then_1
      (bind _aswbp_3dicon (Utilities|Casting|CastToWBP_3DIcon (UserInterface|GetWidget (Variables|Default|GetWidget))))
      (Variables|Default|SetAs%20WBP%203DIcon _aswbp_3dicon)
      (Default|SetUIData _aswbp_3dicon (.name _cameradata) (.icon _cameradata) self))))

(event Collision|EventActorBeginOverlap
  (params (OtherActor :type Actor%20Object%20Reference)))

(event EventTick
  (params (DeltaSeconds :type Float%20%28single-precision%29)))

(fn ConstructionScript
  (CallFunction|SetCameraData))

(fn SetCameraData
  (Variables|/Script/Engine.SpringArmComponent|SetTargetArmLength (Variables|Default|GetSpringArm) (.armlen (Variables|Default|GetCameraData)))
  (Transformation|SetRelativeRotation (Variables|Default|GetSpringArm) (Math|Rotator|MakeRotator 0.0 (.pitch (.rotation (Variables|Default|GetCameraData))) (.yaw (.rotation (Variables|Default|GetCameraData)))) false false)
  (Variables|Default|SetCameraData (Utilities|Struct|MakeCameraData (.name (Variables|Default|GetCameraData)) (Transformation|GetActorLocation) (Math|Rotator|MakeRotator 0.0 (.pitch (.rotation (Variables|Default|GetCameraData))) (.yaw (.rotation (Variables|Default|GetCameraData)))) (.armlen (Variables|Default|GetCameraData)) (.icon (Variables|Default|GetCameraData)))))

(fn ClickIcon
  (bind _cameradata (Variables|Default|GetCameraData))
  (bind _as_bp_pawn (Variables|Default|GetAs%20BP%20Pawn))
  (CallFunction|PlayMedia)
  (Variables|/Game/GamePlay/Game/BP_Pawn.BP_Pawn_C|SetNewCameraData _as_bp_pawn (Utilities|Struct|MakeCameraData (.name _cameradata) (.location _cameradata) (Transformation|GetWorldRotation (Variables|Default|GetSpringArm)) (.armlen _cameradata) (.icon _cameradata)))
  (Variables|/Game/GamePlay/Game/BP_Pawn.BP_Pawn_C|SetCameraNewLen _as_bp_pawn (.armlen _cameradata))
  (Default|Foucs _as_bp_pawn))

(fn PlayMedia
  (if (== (Variables|Default|GetMedia%20Source) 0)
    (Development|PrintString "没有监控视频")
    (else
      (bind _aswbp_3ddetails (Utilities|Casting|CastToWBP_3DDetails (UserInterface|GetWidget (Variables|Default|GetMedia_Widget))))
      (Default|PlayMedia _aswbp_3ddetails (Variables|Default|GetMedia%20Source) self)
      (Rendering|SetVisibility (Variables|Default|GetWidget) false false)))
  (return))

(fn EndMedia
  (bind _aswbp_3ddetails (Utilities|Casting|CastToWBP_3DDetails (UserInterface|GetWidget (Variables|Default|GetMedia_Widget))))
  (Default|EndMedia _aswbp_3ddetails)
  (Rendering|SetVisibility (Variables|Default|GetMedia_Widget) true false))
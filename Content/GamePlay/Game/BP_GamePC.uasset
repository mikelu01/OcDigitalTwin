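; BP_GamePC is a player controller that handles mouse button state and look rotation.
; Left and right mouse press and release events set the MouseLeft and MouseRight flags, which are not read in this Blueprint.
; The LookUpRate and TurnRate axis events share one SetControlRotation call that adds scaled axis input to the current pitch and yaw and zeroes roll.
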(event EventBeginPlay)

(event EventTick
  (params (DeltaSeconds :type Float%20%28single-precision%29)))

(event Input|AxisEvents|InputAxisLookUpRate
  (params (AxisValue :type Float%20%28single-precision%29))
  (bind _returnvalue (Pawn|GetControlRotation :!class /Script/Engine.Controller))
  (Pawn|SetControlRotation (Math|Rotator|MakeRotator 0.0 (+ (* AxisValue 2.0) (.pitch _returnvalue)) (+ (* (stale Input|AxisEvents|InputAxisTurnRate AxisValue) 2.0) (.yaw _returnvalue)))))

(event Input|AxisEvents|InputAxisTurnRate
  (params (AxisValue :type Float%20%28single-precision%29))
  (bind _returnvalue (Pawn|GetControlRotation :!class /Script/Engine.Controller))
  (Pawn|SetControlRotation (Math|Rotator|MakeRotator 0.0 (+ (* (stale Input|AxisEvents|InputAxisLookUpRate AxisValue) 2.0) (.pitch _returnvalue)) (+ (* AxisValue 2.0) (.yaw _returnvalue)))))

(event Input|MouseEvents|RightMouseButton
  (params (Key :type Key%20Structure :default "None"))
  (:Pressed
    (Variables|Default|SetMouse_Right true))
  (:Released
    (Variables|Default|SetMouse_Right false)))

(event Input|MouseEvents|LeftMouseButton
  (params (Key :type Key%20Structure :default "None"))
  (:Pressed
    (Variables|Default|SetMouse_Left true))
  (:Released
    (Variables|Default|SetMouse_Left false)))

(fn ConstructionScript)